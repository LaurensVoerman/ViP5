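; Liquid droplet actor, a short-lived translucent dark blue mesh that falls as a simulated physics body.
; The construction script tints the materials and, when LifeTime is positive, starts a one-shot timer and enables gravity-driven physics with an overlap-only profile and heavy linear damping.
; A SelfDestruct function destroys the actor, while the event graph holds only inactive default events.
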(event EventBeginPlay
  (|CallParentFunction) ; This node is disabled and will not be called.\nDrag off pins to build functionality.
)

(event Collision|EventActorBeginOverlap
  (params (OtherActor :type Actor%20Object%20Reference)))

(event EventTick
  (params (DeltaSeconds :type Float%20%28single-precision%29))
  (|CallParentFunction DeltaSeconds) ; This node is disabled and will not be called.\nDrag off pins to build functionality.
)

(fn ConstructionScript
  (bind _staticmeshcomponent (Variables|Default|GetStaticMeshComponent))
  (bind _lifetime (Variables|Default|GetLifeTime))
  (bind _staticmeshcomponent_2 (Variables|Default|GetStaticMeshComponent))
  (|CallParentFunction)
  (Rendering|Material|SetVectorParameterValueonMaterials _staticmeshcomponent "Color" "0.020000,0.030000,0.220000")
  (Rendering|Material|SetScalarParameterValueonMaterials _staticmeshcomponent "Opacity" 0.8)
  (if (> _lifetime 0.0)
    (Utilities|Time|SetTimerbyEvent (EventDispatchers|CreateEvent :!event SelfDestruct) _lifetime)
    (Physics|SetSimulatePhysics _staticmeshcomponent_2 false)
    (Collision|SetCollisionEnabled _staticmeshcomponent_2 "QueryAndPhysics")
    (Collision|SetCollisionProfileName _staticmeshcomponent_2 "OverlapAll" false :!class /Script/Engine.PrimitiveComponent)
    (Class|PrimitiveComponent|SetLinearDamping _staticmeshcomponent_2 2e+01)
    (Physics|SetSimulatePhysics _staticmeshcomponent_2 true)
    (Physics|SetEnableGravity _staticmeshcomponent_2 true)))

(fn SelfDestruct
  (Actor|DestroyActor))