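; Dropping funnel glassware that holds liquid and releases it drop by drop into the actor connected at its "yellow.in" socket.
; SocketValueChanged sets stopcock flow area or liquid volume, and Tick turns flow and liquid height into a growing hanging droplet, spawning falling BP_LiquidDroplets past a threshold.
; SetLiquidVolume maps volume to level, driving fill materials and a tilt-compensated surface disc.
; GenerateSurface, not called here, builds a procedural surface by plane-cutting a lathed profile.
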(event EventBeginPlay
  (|CallParentFunction) ; This node is disabled and will not be called.\nDrag off pins to build functionality.
)

(event Collision|EventActorBeginOverlap
  (params (OtherActor :type Actor%20Object%20Reference)))

(event EventTick
  (params (DeltaSeconds :type Float%20%28single-precision%29))
  (bind _returnvalue (Math|Float|MakeLiteralFloat 0.005))
  (bind _returnvalue_2 (Math|Float|MakeLiteralFloat 1e+01))
  (bind _flowarea (Variables|Default|GetFlowArea))
  (bind _liquidlevel (Variables|Default|GetLiquidLevel))
  (bind _droplet (Variables|Default|GetDroplet))
  (bind _returnvalue_3 (- 10.4 _liquidlevel))
  (bind _returnvalue_4 (- 0.0 _returnvalue_2))
  (bind _returnvalue_5 (* _returnvalue_3 1e+01))
  (bind _returnvalue_6 (* DeltaSeconds _flowarea _returnvalue_5))
  (|CallParentFunction DeltaSeconds)
  (CallFunction|SetLiquidVolume (Variables|Default|GetLiquidVolume)) ; volume.in
  (if (> _returnvalue_6 0.0)
    (bind _output_get (Variables|Default|SetDropletVolume (+ (Variables|Default|GetDropletVolume) _returnvalue_6)))
    (Variables|Default|SetLiquidVolume (- (Variables|Default|GetLiquidVolume) _returnvalue_6))
    (if (> (- (- _output_get (Math|Float|MakeLiteralFloat 0.05)) _returnvalue) 0.0)
      (bind _returnvalue_7 (CallFunction|GetActorAttachedtoSocket (Utilities|Name|MakeLiteralName "yellow.in")))
      (bind _returnvalue_8 (Game|SpawnActorfromClass "/Game/glassware/RB_flasks/vultrechterB/BP_LiquidDroplet.BP_LiquidDroplet_C" (Math|Transform|MakeTransform (Transformation|GetSocketLocation (Variables|Default|GetStaticMeshComponent) "droplet") "0, 0, 0" (Math|Vector|MakeVector (* (Math|Float|Power (* (- _output_get _returnvalue) 0.238732) 0.333333) 0.02) (* (Math|Float|Power (* (- _output_get _returnvalue) 0.238732) 0.333333) 0.02) (* (Math|Float|Power (* (- _output_get _returnvalue) 0.238732) 0.333333) 0.02))) "Undefined" _returnvalue_7 0.3 _returnvalue_7 0))
      (Physics|SetPhysicsLinearVelocity (Variables|/Script/Engine.StaticMeshActor|GetStaticMeshComponent _returnvalue_8) (Math|Vector|MakeVector (Math|Random|RandomFloatinRange _returnvalue_4 _returnvalue_2) (Math|Random|RandomFloatinRange _returnvalue_4 _returnvalue_2) 0.0) false "None")
      (Variables|Default|SetDropletVolume _returnvalue))
    (Utilities|IsValid _droplet
      (:Is%20Valid
        (Transformation|SetActorRelativeTransform _droplet (Math|Transform|MakeTransform "0, 0, 0" "0, 0, 0" (Math|Vector|MakeVector (* (Math|Float|Power (* (Variables|Default|GetDropletVolume) 0.238732) 0.333333) 0.02) (* (Math|Float|Power (* (Variables|Default|GetDropletVolume) 0.238732) 0.333333) 0.02) (* (Math|Float|Power (* (Variables|Default|GetDropletVolume) 0.238732) 0.333333) 0.02))) false true))
      (:Is%20Not%20Valid
        (Transformation|SetActorRelativeTransform _droplet (Math|Transform|MakeTransform "0, 0, 0" "0, 0, 0" (Math|Vector|MakeVector (* (Math|Float|Power (* (Variables|Default|GetDropletVolume) 0.238732) 0.333333) 0.02) (* (Math|Float|Power (* (Variables|Default|GetDropletVolume) 0.238732) 0.333333) 0.02) (* (Math|Float|Power (* (Variables|Default|GetDropletVolume) 0.238732) 0.333333) 0.02))) false true)))))

(fn ConstructionScript
  (|CallParentFunction)
  (CallFunction|SetLiquidVolume (Variables|Default|GetLiquidVolume)))

(fn SetLiquidVolume
  (params (NewVolume :type Float%20%28single-precision%29))
  (bind _returnvalue (Math|Float|MakeLiteralFloat 1.0))
  (bind _staticmeshcomponent (Variables|Default|GetStaticMeshComponent))
  (bind _returnvalue_2 (Transformation|GetWorldTransform _staticmeshcomponent))
  (bind _returnvalue_3 (Math|Vector|GetUpVector _staticmeshcomponent))
  (bind _rotation (Math|Transform|BreakTransform _returnvalue_2))
  (bind _returnvalue_4 (Class|KismetMathLibrary|NegateRotator _rotation))
  (bind _output_get (Variables|Default|SetLiquidVolume NewVolume))
  (Variables|Default|SetLiquidLevel (select (> NewVolume 2e+01) (+ (* _output_get -0.11) 7.76) (+ (* _output_get -0.242) 10.4)))
  (Rendering|Material|SetScalarParameterValueonMaterials (Variables|Default|Getvultrechter_yellowR_100ml_1_resevoir_outside_R19) "LiquidLevel" (Math|Float|MakeLiteralFloat (+ (Variables|Default|GetLiquidLevel) (* (Math|Float|MakeLiteralFloat -7.5) (- 1.0 (.Z (Math|Vector|BreakVector (Math|Vector|GetUpVector (Variables|Default|GetStaticMeshComponent)))))))))
  (Rendering|Material|SetScalarParameterValueonMaterials (Variables|Default|Getvultrechter_yellowR_100ml_1_resevoir_inside_R18) "LiquidLevel" (Math|Float|MakeLiteralFloat (+ (Variables|Default|GetLiquidLevel) (* (Math|Float|MakeLiteralFloat -7.5) (- 1.0 (.Z (Math|Vector|BreakVector (Math|Vector|GetUpVector (Variables|Default|GetStaticMeshComponent)))))))))
  (Transformation|SetRelativeTransform (Variables|Default|Getsurface_Circle) (Math|Transform|MakeTransform (Math|Vector|MakeVector 0.0 0.0 (+ (/ (- 7.5 (Variables|Default|GetLiquidLevel)) (.Z (Math|Vector|BreakVector _returnvalue_3))) 2e+01)) _returnvalue_4 (Math|Vector|MakeVector (/ _returnvalue (Math|Vector|VectorLengthXY (Math|Vector|RotateVector "1.000000, 0, 0" _returnvalue_4))) (/ _returnvalue (Math|Vector|VectorLengthXY (Math|Vector|RotateVector "0.000000,1.000000,0.000000" _returnvalue_4))) 1.0)) false false)
  (Rendering|Material|SetScalarParameterValueonMaterials (Variables|Default|Getsurface_Circle) "R_MAX" 3.24)
  (Rendering|Material|SetVectorParameterValueonMaterials (Variables|Default|Getsurface_Circle) "UpVector" _returnvalue_3)
  (Rendering|Material|SetScalarParameterValueonMaterials (Variables|Default|Getsurface_Circle) "Height" (+ (/ (- 7.5 (Variables|Default|GetLiquidLevel)) (.Z (Math|Vector|BreakVector _returnvalue_3))) 3.5))
  (Rendering|SetTranslucencySortDistanceOffset (Variables|Default|Getsurface_Circle) -1.0))

(fn SocketValueChanged
  (params (Index :type Integer) (ValueChange :type Float%20%28single-precision%29))
  (bind _self self)
  (bind (_newvalue _minval _maxval) (|CallParentFunction Index ValueChange))
  (Utilities|FlowControl|Sequence
    (:then_0
      (switch int Index
        (:2
          (bind _output_get (Variables|Default|SetFlowArea (* (- 1.0 (Math|Float|Square (Math|Float|Clamp(Float) (* (Math|Float|%(Float) (Math|Float|Absolute(Float) (* _newvalue 2.0)) 1.0) 1e+01)))) 0.1)))
          (if (and (> _output_get 0.0) (> (Variables|Default|GetLiquidVolume) (Math|Float|MakeLiteralFloat 0.005)))
            (Utilities|IsValid (Variables|Default|GetDroplet)
              (:Is%20Valid
                _)
              (:Is%20Not%20Valid
                (bind _returnvalue (Game|SpawnActorfromClass "/Game/glassware/RB_flasks/vultrechterB/BP_LiquidDroplet.BP_LiquidDroplet_C" (Math|Transform|MakeTransform "0, 0, 0") "Undefined" _self 0.0 _self 0))
                (bind _output_get_2 (Variables|Default|SetDroplet _returnvalue))
                (bind _output_get_3 (Variables|Default|SetDropletVolume 0.005))
                (CallFunction|SetLiquidVolume (- (Variables|Default|GetLiquidVolume) _output_get_3)) ; volume.in
                (Transformation|AttachActorToActor _output_get_2 self "droplet" "KeepRelative" "KeepRelative" "KeepRelative" true)))
            (Transformation|SetActorRelativeTransform (Variables|Default|GetDroplet) (Math|Transform|MakeTransform "0, 0, 0" "0, 0, 0" (Math|Vector|MakeVector (* (Math|Float|Power (* (Variables|Default|GetDropletVolume) 0.238732) 0.333333) 0.01) (* (Math|Float|Power (* (Variables|Default|GetDropletVolume) 0.238732) 0.333333) 0.01) (* (Math|Float|Power (* (Variables|Default|GetDropletVolume) 0.238732) 0.333333) 0.01))) false true)))
        (:3
          (CallFunction|SetLiquidVolume _newvalue) ; volume.in
        )))
    (:then_1
      (return _newvalue _minval _maxval))))

(fn GenerateSurface
  (params (Normal :type Vector) (Level :type Float%20%28single-precision%29))
  (bind _returnvalue (Math|Vector|MakeVector 0.0 0.0 17.5))
  (bind _verts (LocalVariables|Getverts))
  (bind _triangles (LocalVariables|GetTriangles))
  (bind _triangles_2 (LocalVariables|GetTriangles))
  (bind _trianglesback (LocalVariables|GetTrianglesBack))
  (bind _verts_2 (LocalVariables|Getverts))
  (bind _returnvalue_2 (Utilities|Array|Length _triangles))
  (bind _returnvalue_3 (> _returnvalue_2 0))
  (bind _output_get (LocalVariables|Set_Normal Normal))
  (LocalVariables|Set_Level Level)
  (Utilities|Array|Clear (LocalVariables|Getverts))
  (LocalVariables|SetLathe (Utilities|Array|MakeArray (- (Math|Vector|MakeVector 0.0 0.0 7.1) _returnvalue) (- (Math|Vector|MakeVector 0.2 0.0 7.1) _returnvalue) (- (Math|Vector|MakeVector 1.8 0.0 11.3) _returnvalue) (- (Math|Vector|MakeVector 1.8 0.0 24.200001) _returnvalue) (- (Math|Vector|MakeVector 0.585 0.0 25.6) _returnvalue)))
  (for _index (range 0 36)
    (LocalVariables|Set_prevVertexLevel (- (Math|Vector|DotProduct (Utilities|Array|Get(acopy) (LocalVariables|GetLathe)) (LocalVariables|Get_Normal)) (LocalVariables|Get_Level)))
    (bind (_array_element _array_index) (Utilities|Array|ForEachLoopwithBreak (LocalVariables|GetLathe))
      (:LoopBody
        (LocalVariables|Set_currVertexLevel (- (Math|Vector|DotProduct _array_element (LocalVariables|Get_Normal)) (LocalVariables|Get_Level)))
        (if (< (* (- (Math|Vector|DotProduct _array_element (LocalVariables|Get_Normal)) (LocalVariables|Get_Level)) (LocalVariables|Get_prevVertexLevel)) 0.0)
          (Utilities|Array|Add (LocalVariables|Getverts) (+ _array_element (* (- (Utilities|Array|Get(acopy) (LocalVariables|GetLathe) (- _array_index 1)) _array_element) (/ (LocalVariables|Get_currVertexLevel) (- (LocalVariables|Get_currVertexLevel) (LocalVariables|Get_prevVertexLevel)))))))
        (LocalVariables|Set_prevVertexLevel (LocalVariables|Get_currVertexLevel)))
      (:Completed
        (bind (_array_element_2 _array_index_2) (Utilities|Array|ForEachLoopwithBreak (LocalVariables|GetLathe))
          (:LoopBody
            (if (< (* (- (Math|Vector|DotProduct _array_element_2 (LocalVariables|Get_Normal)) (LocalVariables|Get_Level)) (- (Math|Vector|DotProduct (Math|Vector|RotateVector _array_element_2 (Math|Rotator|MakeRotator 0.0 0.0 1e+01)) (LocalVariables|Get_Normal)) (LocalVariables|Get_Level))) 0.0)
              (Utilities|Array|Add (LocalVariables|Getverts) (+ _array_element_2 (* (- _array_element_2 (Math|Vector|RotateVector _array_element_2 (Math|Rotator|MakeRotator 0.0 0.0 1e+01))) (/ (- (Math|Vector|DotProduct _array_element_2 (LocalVariables|Get_Normal)) (LocalVariables|Get_Level)) (- (- (Math|Vector|DotProduct _array_element_2 (LocalVariables|Get_Normal)) (LocalVariables|Get_Level)) (- (Math|Vector|DotProduct (Math|Vector|RotateVector _array_element_2 (Math|Rotator|MakeRotator 0.0 0.0 1e+01)) (LocalVariables|Get_Normal)) (LocalVariables|Get_Level))))))))
            (Utilities|Array|SetArrayElem (LocalVariables|GetLathe) _array_index_2 (Math|Vector|RotateVector _array_element_2 (Math|Rotator|MakeRotator 0.0 0.0 1e+01))))))))
  (for (_ _array_index_3) (LocalVariables|Getverts)
    (if (> _array_index_3 1)
      (Utilities|Array|Add _triangles_2 0)
      (Utilities|Array|Add _triangles_2 _array_index_3)
      (Utilities|Array|Add _triangles_2 (- _array_index_3 1))
      (Utilities|Array|Add _trianglesback 0)
      (Utilities|Array|Add _trianglesback (- _array_index_3 1))
      (Utilities|Array|Add _trianglesback _array_index_3)))
  (Class|ProceduralMeshComponent|SetMeshSectionVisible (Variables|Default|GetSurface) 0 _returnvalue_3)
  (if _returnvalue_3
    (Utilities|FlowControl|Sequence
      (:then_0
        ;[1 1 1] add degenerate triangle for sorting
        (bind _returnvalue_4 (Utilities|Array|Add _verts (Utilities|Array|Get(acopy) (LocalVariables|GetLathe))))
        (bind _returnvalue_5 (Utilities|Array|Add _verts (Utilities|Array|Get(acopy) (LocalVariables|GetLathe) (- (Utilities|Array|Length (LocalVariables|GetLathe)) 1))))
        (Utilities|Array|Add (LocalVariables|GetTriangles) _returnvalue_4)
        (Utilities|Array|Add (LocalVariables|GetTriangles) _returnvalue_5)
        (Utilities|Array|Add (LocalVariables|GetTriangles) _returnvalue_5))
      (:then_1
        (for _array_element_3 _verts_2
          (Utilities|Array|Add (LocalVariables|GetvertexNormals) (LocalVariables|Get_Normal)))
        (Class|ProceduralMeshComponent|CreateMeshSectionLinearColor (Variables|Default|GetSurface) 0 _verts_2 (LocalVariables|GetTriangles) (LocalVariables|GetvertexNormals) 0 0 0 0 0 0 false)
        (Rendering|Material|SetMaterial (Variables|Default|GetSurface) 0 "/Game/glassware/_materials/M_plastic_red.M_plastic_red")
        (for (_array_element_4 _array_index_4) (LocalVariables|GetvertexNormals)
          (Utilities|Array|SetArrayElem (LocalVariables|GetvertexNormals) _array_index_4 (- "0, 0, 0" _array_element_4))
          (Class|ProceduralMeshComponent|CreateMeshSectionLinearColor (Variables|Default|GetSurface) 1 (LocalVariables|Getverts) (LocalVariables|GetTrianglesBack) (LocalVariables|GetvertexNormals) 0 0 0 0 0 0 false)
          (Rendering|Material|SetMaterial (Variables|Default|GetSurface) 1 "/Game/glassware/_materials/M_plastic_yellow.M_plastic_yellow"))))))

(fn GetActorAttachedtoSocket
  (params (B :type Name))
  (if (Utilities|Name|Equal(Name) (Variables|Default|GetAttachedSocketName) B)
    (return (Actor|GetParentActor))
    (else
      (bind _outactors (CallFunction|GetAllAttachedActors))
      (for _array_element _outactors
        (if (Utilities|Name|Equal(Name) (Class|Actor|GetAttachParentSocketName _array_element) B)
          (bind _asbp_pickup_cube (Utilities|Casting|CastToBP_PickupCube _array_element))
          (if (not (Utilities|Enum|Equal(Enum) (Class|BlueprintPathsLibrary|GetExtension (Utilities|String|ToString(Name) (Variables|/Game/VirtualRealityBP/Blueprints/BP_PickupCube.BP_PickupCube_C|GetAttachedSocketName _asbp_pickup_cube)) false) "clip"))
            (return _array_element))))
      (return 0))))